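; Cube actor Blueprint that appears to be a simple test of click and touch input.
; A mouse click or touch begin shares one chain that jumps the actor upward with a non-swept world offset, then prints a clicked message.
; Touch enter, BeginPlay, overlap, Tick and the construction script do nothing.
; Disconnected leftover nodes for a sideways move, a touched message and an array insert never run.
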(event `self.ReceiveActorOnInputTouchBegin`
  (params (FingerIndex :type "ETouchIndex Enum" :default "Touch1"))
  (`self.K2_AddActorWorldOffset` (`KismetMathLibrary.MakeVector` 0.0 0.0 333.0) :!label _label)
  (`KismetSystemLibrary.PrintString` (`KismetStringLibrary.Concat_StrStr` "" "I'm clicked!")))

(event `self.ReceiveActorOnClicked`
  (params (ButtonPressed :type "Key Structure" :default "AnyKey"))
  (goto _label))

(event `self.ReceiveActorOnInputTouchEnter`
  (params (FingerIndex :type "ETouchIndex Enum" :default "Touch1")))

(fn `UserConstructionScript`)