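; Touch-input controller for a card battle game, letting the player drag and target their own battle entities.
; A Ready/Drag/Target state machine picks the entity under the cursor, sending pointing spells, hero skills and placed minions straight to targeting.
; Dragged entities follow the raised hit point, and release spawns a pointer actor as the cable's end.
; Target updates, request sending and minion position functions are unfinished stubs.
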(event `InputTouch`
  (params (Location :type "Vector Structure") (FingerIndex :type "ETouchIndex Enum"))
  (bind _state (`self.State`))
  (:`Pressed`
    (switch `/Game/Blueprint/StateRebuilt` _state
      (:`NewEnumerator12`
        (`KismetSystemLibrary.PrintString` "")
        (set `self.OpData` "")
        (bind _hitactor (`self.GetPointedActor`))
        (bind _asbattle_entity (cast `/Game/Blueprint/BattleEntity` _hitactor))
        (if (`/Game/Blueprint/BattleEntity.isMine` _asbattle_entity)
          (set `self.State` "NewEnumerator13")
          (bind _output_get (set `self.RootOrigin` _asbattle_entity))
          (bind _asspell_card (cast `/Game/Blueprint/SpellCard` _output_get)
            (:`then`
              (if (`/Game/Blueprint/BattleEntity.isPointing` _asspell_card)
                (set `self.State` "NewEnumerator14" :!label _label)
                (if (not (!= (`self.PointingEnd`) null))
                  (bind _hitpos (`self.GetPointedPosition`))
                  (bind _returnvalue (`|SpawnActorFromClass` "/Script/Engine.Actor" (`KismetMathLibrary.Conv_VectorToTransform` (+ _hitpos (`self.UpliftHeight`))) "Undefined" "OverrideRootScale"))
                  (set `self.PointingEnd` _returnvalue))))
            (:`CastFailed`
              (cast `/Game/Blueprint/SkillOfHero` _output_get
                (:`then`
                  (goto _label))
                (:`CastFailed`
                  (cast `/Game/Blueprint/PlacedMinion` _output_get)
                  (goto _label)))))))))
  (:`Released`
    (switch `/Game/Blueprint/StateRebuilt` _state
      (:`NewEnumerator13`
        (`KismetSystemLibrary.PrintString` "")
        (set `self.State` "NewEnumerator14")
        (if (not (!= (`self.PointingEnd`) null))
          (bind _hitpos_2 (`self.GetPointedPosition`))
          (bind _returnvalue_2 (`|SpawnActorFromClass` "/Script/Engine.Actor" (`KismetMathLibrary.Conv_VectorToTransform` (+ _hitpos_2 (`self.UpliftHeight`))) "Undefined" "OverrideRootScale"))
          (set `self.PointingEnd` _returnvalue_2)
          (bind _cableorigin (`/Game/Blueprint/BattleEntity.DragStateEndProcess` (`self.RootOrigin`)))
          (set `self.CableOrigin` _cableorigin)
          (`CableComponent.SetAttachEndTo` (`/Game/Blueprint/BattleEntity.BECable` (`self.CableOrigin`)) (`self.PointingEnd`) "None")))
      (:`NewEnumerator14`
        (`KismetSystemLibrary.PrintString` "not implemented! from target state to request!"))))
  (:`Moved`
    (switch `/Game/Blueprint/StateRebuilt` _state
      (:`NewEnumerator13`
        (`KismetSystemLibrary.PrintString` "not implemented! in drag state!")
        (bind _hitpos_3 (`self.GetPointedPosition`))
        (`self.K2_SetActorLocation` (`self.RootOrigin`) (+ _hitpos_3 (`self.UpliftHeight`)) false false)
        (`/Game/Blueprint/BattleEntity.OnDragged` (`self.RootOrigin`)))
      (:`NewEnumerator14`
        (`KismetSystemLibrary.PrintString` "not implemented! should get the cable! ")))))

(fn `GetPointedActor`
  (returns (HitActor :type "Actor Object Reference"))
  (return (`.HitActor` (`GameplayStatics.BreakHitResult` (`self.GetHitResultUnderCursorByChannel` self "TraceTypeQuery1" true)))))

(fn `GetPointedPosition`
  (returns (HitPos :type "Vector Structure"))
  (return (`.Location` (`GameplayStatics.BreakHitResult` (`self.GetHitResultUnderCursorByChannel` self "TraceTypeQuery1" true)))))

(fn `RemoveMinion`
  (params (index :type Integer) (`MyT-OppF` :type Boolean)))

(fn `sendOpRequest`
  ;[1 1 1] 需要实现post/resp逻辑
  (set `self.State` "NewEnumerator12")
  (set `self.State` "NewEnumerator12")
  (return))

(fn `setMyMinionPos`)

(fn `setOppMinionPos`)

(fn `UserConstructionScript`
  (set `self.State` "NewEnumerator12"))