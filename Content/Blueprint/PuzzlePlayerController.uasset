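; Player controller for a turn-based card battler, turning touch input into minion, card and hero-skill interactions; largely an unfinished skeleton.
; A press traces under the cursor, classifies the battle entity and sets a targeting or drag state, recording origins for targeting.
; Release and move switch on the MyTurnReadyState constant rather than State, with move branches empty.
; Minion-card spawning is disconnected, and positioning, removal and server requests are stubs.
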(event `InputTouch`
  (params (Location :type "Vector Structure") (FingerIndex :type "ETouchIndex Enum"))
  (bind _newminion (`self.newMinion`))
  (:`Pressed`
    (switch `/Game/Blueprint/StateEnum` (`self.State`)
      (:`NewEnumerator1`
        (bind _hitactor (`self.GetPointedActor`))
        ;[1 1 1] 检视actor类型，暂时忽略英雄自己的物理攻击情况
        (bind _output_get (set `self.ActorPointed` _hitactor))
        (bind _asbattle_entity (cast `/Game/Blueprint/BattleEntity` _output_get))
        (set `self.RootOrigin` _asbattle_entity)
        (cast `/Game/Blueprint/PlacedMinion` _asbattle_entity
          (:`then`
            (set `self.State` "NewEnumerator2"))
          (:`CastFailed`
            (bind _asminion_card (cast `/Game/Blueprint/MinionCard` _asbattle_entity)
              (:`CastFailed`
                (bind _asspell_card (cast `/Game/Blueprint/SpellCard` _asbattle_entity)
                  (:`then`
                    (if (`/Game/Blueprint/BattleEntity.isPointing` _asspell_card)
                      (set `self.CableOrigin` _asbattle_entity)
                      (set `self.State` "NewEnumerator10")
                      (else
                        (set `self.State` "NewEnumerator7"))))
                  (:`CastFailed`
                    (bind _asskill_of_hero (cast `/Game/Blueprint/SkillOfHero` _asbattle_entity))
                    (if (`/Game/Blueprint/BattleEntity.isPointing` _asskill_of_hero)
                      (set `self.CableOrigin` _asbattle_entity)
                      (set `self.State` "NewEnumerator6")))))))))))
  (:`Released`
    ;[1 1 1] todo武器还未处理
    (switch `/Game/Blueprint/StateEnum` "NewEnumerator1"
      (:`NewEnumerator3`
        ;[1 1 1] todo设置为假时的容错
        (if (!= _newminion null)
          (`/Game/Blueprint/PlacedMinion.setFullyPlaced` _newminion)
          (set `self.State` "NewEnumerator1")))))
  (:`Moved`
    (switch `/Game/Blueprint/StateEnum` "NewEnumerator1"
      (:`NewEnumerator3`
        (if true
          _))
      (:`NewEnumerator7`
        (if true
          _))
      (:`NewEnumerator2`
        (if true
          _))
      (:`NewEnumerator6`
        (if true
          _))
      (:`NewEnumerator10`
        (if true
          _))
      (:`NewEnumerator11`
        (if true
          _)))))

(fn `GetPointedActor`
  (returns (HitActor :type "Actor Object Reference"))
  (return (`.HitActor` (`GameplayStatics.BreakHitResult` (`self.GetHitResultUnderCursorByChannel` self "TraceTypeQuery1" true)))))

(fn `GetPointedPosition`
  (returns (HitPos :type "Vector Structure"))
  (return (`.Location` (`GameplayStatics.BreakHitResult` (`self.GetHitResultUnderCursorByChannel` self "TraceTypeQuery1" true)))))

(fn `RemoveMinion`
  (params (index :type Integer) (`MyT-OppF` :type Boolean)))

(fn `sendOpRequest`
  ;[1 1 1] 需要实现post/resp逻辑
  (set `self.State` "NewEnumerator8")
  (set `self.State` "NewEnumerator1")
  (return))

(fn `setMyMinionPos`)

(fn `setOppMinionPos`)

(fn `UserConstructionScript`)